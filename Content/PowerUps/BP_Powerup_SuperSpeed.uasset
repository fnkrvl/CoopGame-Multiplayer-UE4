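; Super speed powerup that temporarily doubles the movement speed of the player it activates for.
; On activation it stores that player and sets the Character Movement component's MaxWalkSpeed to twice the current GetMaxSpeed value.
; On expiry it sets MaxWalkSpeed to half of GetMaxSpeed if the player is still valid, then calls the parent expiry logic.
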(event `self.OnActivated`
  (params (ActiveFor :type "Actor Object Reference"))
  (bind _returnvalue (`self.GetComponentByClass` ActiveFor "/Script/Engine.CharacterMovementComponent"))
  (set `self.Active For Player` ActiveFor)
  (set `CharacterMovementComponent.MaxWalkSpeed` (* (`MovementComponent.GetMaxSpeed` _returnvalue) 2.0) _returnvalue))

(event `self.OnExpired`
  (bind _active_for_player (`self.Active For Player`))
  (bind _returnvalue (`self.GetComponentByClass` _active_for_player "/Script/Engine.CharacterMovementComponent"))
  (`/Engine/EditorBlueprintResources/StandardMacros.IsValid` _active_for_player
    (:`Is Valid`
      (set `CharacterMovementComponent.MaxWalkSpeed` (/ (`MovementComponent.GetMaxSpeed` _returnvalue) 2.0) _returnvalue))
    (:`Is Not Valid`
      _))
  (`parent.OnExpired`))

(fn `UserConstructionScript`)